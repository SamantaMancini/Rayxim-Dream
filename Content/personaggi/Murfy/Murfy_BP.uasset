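; Murfy is a character Blueprint that turns to face the player once on BeginPlay and exposes events for its emotional reactions.
; Speak, Worry, Angry and Sad play looping animations directly on the mesh, sequenced with timed delays.
; Speak and Sad return to idle, Worry keeps looping, and Angry briefly plays the speak animation before the angry one, then destroys the actor.
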(event `self.ReceiveBeginPlay`
  (bind (_returnvalue_roll _returnvalue_pitch _returnvalue_yaw) (`KismetMathLibrary.BreakRotator` (`KismetMathLibrary.FindLookAtRotation` (`self.K2_GetActorLocation`) (`self.K2_GetActorLocation` (`GameplayStatics.GetPlayerCharacter` 0)))))
  (`self.K2_SetActorRotation` (`KismetMathLibrary.MakeRotator` _returnvalue_roll 0.0 _returnvalue_yaw)))

(event `Speak`
  (bind _mesh (`self.Mesh`))
  (`SkeletalMeshComponent.PlayAnimation` _mesh "/Game/personaggi/Murfy/murfy_Anim_Murfy_arm_speak_001.murfy_Anim_Murfy_arm_speak_001" true)
  (`KismetSystemLibrary.Delay` 2.0)
  (`SkeletalMeshComponent.PlayAnimation` _mesh "/Game/personaggi/Murfy/murfy_Anim_Murfy_arm_Idle.murfy_Anim_Murfy_arm_Idle" true))

(event `Worry`
  (`SkeletalMeshComponent.PlayAnimation` (`self.Mesh`) "/Game/personaggi/Murfy/murfy_Anim_Murfy_arm_worry.murfy_Anim_Murfy_arm_worry" true))

(event `Angry`
  (bind _mesh (`self.Mesh`))
  (`SkeletalMeshComponent.PlayAnimation` _mesh "/Game/personaggi/Murfy/murfy_Anim_Murfy_arm_speak_001.murfy_Anim_Murfy_arm_speak_001" true)
  (`KismetSystemLibrary.Delay` 0.5)
  (`SkeletalMeshComponent.PlayAnimation` _mesh "/Game/personaggi/Murfy/Angry.Angry" true)
  (`KismetSystemLibrary.Delay` 1.5)
  (`self.K2_DestroyActor`))

(event `Sad`
  (bind _mesh (`self.Mesh`))
  (`SkeletalMeshComponent.PlayAnimation` _mesh "/Game/personaggi/Murfy/Sad.Sad" true)
  (`KismetSystemLibrary.Delay` 2.0)
  (`SkeletalMeshComponent.PlayAnimation` _mesh "/Game/personaggi/Murfy/murfy_Anim_Murfy_arm_Idle.murfy_Anim_Murfy_arm_Idle" true))

(fn `UserConstructionScript`)