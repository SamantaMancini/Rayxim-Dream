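; Teensie character Blueprint that turns to face the player and can spawn a collectable at its position.
; Each Tick, it applies only the yaw of a look-at rotation toward player 0's character, keeping pitch and roll at zero.
; The Collectables function spawns the passed class at the Teensie's location, leaving its Index and Collected inputs unused.
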(event `self.ReceiveBeginPlay`)

(event `self.ReceiveTick`
  (params (DeltaSeconds :type "Float (single-precision)"))
  (bind _returnvalue (`GameplayStatics.GetPlayerCharacter` 0))
  (`/Engine/EditorBlueprintResources/StandardMacros.IsValid` _returnvalue
    (:`Is Valid`
      (`self.K2_SetActorRotation` (`KismetMathLibrary.MakeRotator` 0.0 0.0 (.yaw (`KismetMathLibrary.FindLookAtRotation` (`self.K2_GetActorLocation`) (`self.K2_GetActorLocation` _returnvalue))))))))

(fn `Collectables`
  (params (Index :type Integer) (Collected :type Boolean) (Class :type "Actor Class Reference"))
  (`|SpawnActorFromClass` Class (`KismetMathLibrary.MakeTransform` (`self.K2_GetActorLocation`)) "Undefined" "OverrideRootScale" null null)
  (return))

(fn `UserConstructionScript`)