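; TeensieCrownBP is a short-lived Teensie crown that animates, registers a Yellowlum collectable and then removes itself.
; On BeginPlay it runs a timed chain of delays: it plays the Lum montage, calls Collectables to mark the Yellowlum as collected, then destroys the actor.
; Overlap and Tick are disabled stubs, so spawning alone drives the sequence, with no player contact check.
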(event `self.ReceiveBeginPlay`
  (`parent.ReceiveBeginPlay`)
  (`KismetSystemLibrary.Delay` 0.5)
  (`self.PlayAnimMontage` "/Game/personaggi/Teensie/TeensieCrown/Lum.Lum")
  (`KismetSystemLibrary.Delay` 0.5)
  (`self.Collectables` 1 true "/Game/ThirdPersonBP/Yellow_green_red_lum/Yellowlum.Yellowlum_C")
  (`KismetSystemLibrary.Delay` 1.0)
  (`self.K2_DestroyActor`))

(fn `UserConstructionScript`
  (`parent.UserConstructionScript`))