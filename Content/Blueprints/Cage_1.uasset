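; Breakable cage actor that counts as a rescued cage in Rayxim_GameMode when damaged by a simpleattackBP1.
; On that hit it stops its HelpitchCue audio, plays an explosion sound, spawns a Yellowlum at its mesh location and destroys itself.
; It adds its own Cage widget to the viewport on BeginPlay and plays that widget's animation when destroyed.
; A cutscene branch with input disabling is left unconnected.
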(event `self.ReceiveBeginPlay`
  (bind _returnvalue (`|CreateWidget` "/Game/ThirdPersonBP/Widget_Health_and_level/Cage.Cage_C"))
  (bind _output_get (set `self.gabbia` _returnvalue))
  (`UserWidget.AddToViewport` _output_get 0))

(event `self.ReceiveAnyDamage`
  (params (Damage :type "Float (single-precision)") (DamageType :type "DamageType Object Reference") (InstigatedBy :type "Controller Object Reference") (DamageCauser :type "Actor Object Reference"))
  (cast `/Game/Blueprints/simpleattackBP1_2018-12-15-23-32-02` DamageCauser)
  (`self.CustomEvent_0`)
  (`GameplayStatics.PlaySoundAtLocation` "/Game/Enemies/enemyBosses/EXPLO1.EXPLO1" (0.0 0.0 0.0) (struct) 1.0 1.0 0.0 null null null)
  (bind _asrayxim_game_mode (cast `/Game/ThirdPersonBP/Blueprints/Rayxim_Game_mode/Rayxim_GameMode` (`GameplayStatics.GetGameMode`)))
  (`/Game/ThirdPersonBP/Blueprints/Rayxim_Game_mode/Rayxim_GameMode.Add Cage` _asrayxim_game_mode)
  (`|SpawnActorFromClass` "/Game/ThirdPersonBP/Yellow_green_red_lum/Yellowlum.Yellowlum_C" (`KismetMathLibrary.MakeTransform` (`SceneComponent.K2_GetComponentLocation` (`self.StaticMesh`))) "Undefined" "OverrideRootScale" null null)
  (`self.K2_DestroyActor`))

(event `CustomEvent_0`
  (`AudioComponent.Stop` (`self.helpitch_Cue`)))

(event `Destroy`
  (`self.Cage`))

(event `self.ReceiveDestroyed`
  (`self.Destroy`))

(event `Cage`
  (bind _gabbia (`self.gabbia`))
  (`UserWidget.PlayAnimation` _gabbia (`/Game/ThirdPersonBP/Widget_Health_and_level/Cage.cage` _gabbia) 0.0 1 "Forward" 1.0))

(event `Disable input`
  (bind _asrayxim (cast `/Game/ThirdPersonBP/Rayxim_Animation/Rayxim_2018-12-18-22-44-30` (`GameplayStatics.GetPlayerCharacter` 0)))
  (`self.DisableInput` _asrayxim (`GameplayStatics.GetPlayerController` 0)))

(fn `UserConstructionScript`)