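; Visual indicator actor, named as a map 3 button, that shows the on/off state of a referenced button actor.
; On BeginPlay it binds to that button's on event, then swaps its static mesh material between emissive and plain color according to IsOn.
; A separate Color function, not called within this Blueprint, only prints the game mode's ConteggioButton count for values zero to three.
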(event `self.ReceiveBeginPlay`
  (bind _asbutton (cast `/Game/Blueprints/button` (`self.Actor`)))
  (add `/Game/Blueprints/button.On` _asbutton (delegate `ONButton`)))

(event `ONButton`
  (bind _asbutton (cast `/Game/Blueprints/button` (`self.Actor`)))
  (if (`/Game/Blueprints/button.IsOn` _asbutton)
    (`PrimitiveComponent.SetMaterial` (`self.StaticMeshComponent`) 0 "/Game/Blueprints/emissive_bottone_2018-12-13-19-48-24.emissive_bottone")
    (else
      (`PrimitiveComponent.SetMaterial` (`self.StaticMeshComponent`) 0 "/Game/ThirdPersonBP/Maps/Jungle/BUTTON_COLOR_Mat.BUTTON_COLOR_Mat"))))

(fn `Color`
  (bind _asrayxim_game_mode (cast `/Game/ThirdPersonBP/Blueprints/Rayxim_Game_mode/Rayxim_GameMode` (`GameplayStatics.GetGameMode`)))
  (switch `int` (`/Game/ThirdPersonBP/Blueprints/Rayxim_Game_mode/Rayxim_GameMode.ConteggioButton` _asrayxim_game_mode)
    (:`0`
      (`KismetSystemLibrary.PrintString` "0"))
    (:`1`
      (`KismetSystemLibrary.PrintString` "1"))
    (:`2`
      (`KismetSystemLibrary.PrintString` "2"))
    (:`3`
      (`KismetSystemLibrary.PrintString` "3"))))

(fn `UserConstructionScript`)