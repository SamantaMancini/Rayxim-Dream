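; A one-shot lever prop that plays a Matinee with a camera cut when a simpleattackBP1 actor overlaps it.
; On first overlap, gated by DoOnce before the cast, it plays the lever animation, waits, then starts the Matinee and switches the player's view to the Open target.
; After another short delay it calls CameraOff; a camera_off event blends the view back to the player character.
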(event `camera_off`
  (`PlayerController.SetViewTargetWithBlend` (`GameplayStatics.GetPlayerController` 0) (`GameplayStatics.GetPlayerCharacter` 0) 1.0 "VTBlend_Linear" 0.0 false))

(event `Camera`
  (`PlayerController.SetViewTargetWithBlend` (`GameplayStatics.GetPlayerController` 0) (`self.open`) 0.0 "VTBlend_Linear" 0.0 false))

(event `self.ReceiveActorBeginOverlap`
  (params (OtherActor :type "Actor Object Reference"))
  (`/Engine/EditorBlueprintResources/StandardMacros.DoOnce` false
    (:`Completed`
      (cast `/Game/Blueprints/simpleattackBP1_2018-12-15-23-32-02` OtherActor)
      (`SkeletalMeshComponent.PlayAnimation` (`self.SkeletalMeshComponent`) "/Game/ThirdPersonBP/Maps/Temple/LevaAnim.LevaAnim" false)
      (`KismetSystemLibrary.Delay` 0.8)
      (`MatineeActor.Play` (`self.matinee`))
      (`self.Camera`)
      (`KismetSystemLibrary.Delay` 0.8)
      (`self.camera_off`))))

(fn `UserConstructionScript`)