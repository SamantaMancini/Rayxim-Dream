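; Temple spike trap that repeatedly raises and lowers its spikes and damages the Rayxim that touches it.
; A self-recalling Play event, started on BeginPlay, chains delays with skeletal animations for rising, active and lowering phases.
; It enables collision just before the rise and disables it as the spikes lower.
; Overlaps with that collision apply fixed damage only to actors that cast to Rayxim.
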(event `self.ReceiveBeginPlay`
  (`self.Play`))

(event `Play`
  (bind _skeletalmeshcomponent (`self.SkeletalMeshComponent`))
  (`KismetSystemLibrary.Delay` 1.5)
  (`PrimitiveComponent.SetCollisionEnabled` (`self.Collision`) "QueryAndPhysics")
  (`SkeletalMeshComponent.PlayAnimation` (`self.SkeletalMeshComponent`) "/Game/ThirdPersonBP/Maps/Temple/Objects/Objects_temple_Anim_Spine_up.Objects_temple_Anim_Spine_up" false)
  (`KismetSystemLibrary.Delay` 1.0)
  (`SkeletalMeshComponent.PlayAnimation` _skeletalmeshcomponent "/Game/ThirdPersonBP/Maps/Temple/Objects/Objects_temple_Anim_spina.Objects_temple_Anim_spina" false)
  (`KismetSystemLibrary.Delay` 3.0)
  (`PrimitiveComponent.SetCollisionEnabled` (`self.Collision`) "NoCollision")
  (`SkeletalMeshComponent.PlayAnimation` _skeletalmeshcomponent "/Game/ThirdPersonBP/Maps/Temple/Objects/Objects_temple_Anim_Spine_down.Objects_temple_Anim_Spine_down" false)
  (`PrimitiveComponent.SetCollisionEnabled` (`self.Collision`) "NoCollision")
  (`KismetSystemLibrary.Delay` 5.0)
  (`self.Play`))

(event `self.Collision.OnComponentBeginOverlap`
  (params (OverlappedComponent :type "PrimitiveComponent Object Reference") (OtherActor :type "Actor Object Reference") (OtherComp :type "PrimitiveComponent Object Reference") (OtherBodyIndex :type Integer) (bFromSweep :type Boolean) (SweepResult :type "HitResult Structure (by ref)"))
  (bind _asrayxim (cast `/Game/ThirdPersonBP/Rayxim_Animation/Rayxim_2018-12-18-22-44-30` OtherActor))
  (`GameplayStatics.ApplyDamage` _asrayxim 10.0))

(fn `UserConstructionScript`)