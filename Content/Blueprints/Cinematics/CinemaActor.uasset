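; CinemaActor runs the transformation cinematic that swaps Boss_002 for the SecondFormNymphlix actor.
; Its Transform event disables input on Rayxim, waits briefly, then covers the screen with a FlashWhite widget.
; It then starts the second form, passes it a randomly chosen PathMessage entry and destroys Boss_002, finding each actor by class and using the first instance.
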(event `Transform`
  (bind _outactors (`GameplayStatics.GetAllActorsOfClass` "/Game/ThirdPersonBP/Rayxim_Animation/Rayxim_2018-12-18-22-44-30.Rayxim_C"))
  (`self.DisableInput` (`|GetArrayItem` _outactors) (`GameplayStatics.GetPlayerController` 0))
  (bind _outactors_2 (`GameplayStatics.GetAllActorsOfClass` "/Game/Enemies/enemyBosses/Boss_002/Boss_002.Boss_002_C"))
  (`KismetSystemLibrary.Delay` 0.5)
  (bind _returnvalue (`|CreateWidget` "/Game/Enemies/enemyBosses/Boss_002/texture_secondform/FlashWhite.FlashWhite_C"))
  (`UserWidget.AddToViewport` _returnvalue 0)
  (bind _outactors_3 (`GameplayStatics.GetAllActorsOfClass` "/Game/Enemies/enemyBosses/Boss_002/texture_secondform/SecondFormNymphlix.SecondFormNymphlix_C"))
  (bind _output (`|GetArrayItem` _outactors_3))
  (`/Game/Enemies/enemyBosses/Boss_002/texture_secondform/SecondFormNymphlix.Start` _output)
  (message `/Game/Enemies/EnemyUtilities.Path` _output (`|GetArrayItem` (`self.Array`) (`KismetMathLibrary.RandomIntegerInRange` 0 10)))
  (`self.K2_DestroyActor` (`|GetArrayItem` _outactors_2)))

(fn `UserConstructionScript`)