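; Water_Dirt_BP is a dirty-water hazard that damages the Rayxim player and relocates uovoBP (egg) actors that touch it.
; When Rayxim overlaps the actor, it applies fixed damage, then reads the game mode's Healthbar to call either GameOver or RespawnPlayer.
; When a uovoBP overlaps the static mesh, it spawns a replacement at one of four randomly chosen reference actors and destroys the original.
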(event `self.ReceiveActorBeginOverlap`
  (params (OtherActor :type "Actor Object Reference"))
  (bind _asrayxim (cast `/Game/ThirdPersonBP/Rayxim_Animation/Rayxim_2018-12-18-22-44-30` OtherActor))
  (`GameplayStatics.ApplyDamage` _asrayxim 20.0 null self)
  (if (<= (`/Game/ThirdPersonBP/Blueprints/Rayxim_Game_mode/Rayxim_GameMode.Healthbar` (cast `/Game/ThirdPersonBP/Blueprints/Rayxim_Game_mode/Rayxim_GameMode` (`GameplayStatics.GetGameMode`) :!pure true)) 0)
    (`/Game/ThirdPersonBP/Rayxim_Animation/Rayxim_2018-12-18-22-44-30.Game over` _asrayxim)
    (else
      (`/Game/ThirdPersonBP/Rayxim_Animation/Rayxim_2018-12-18-22-44-30.RespawnPlayer` _asrayxim))))

(event `self.StaticMeshComponent.OnComponentBeginOverlap`
  (params (OverlappedComponent :type "PrimitiveComponent Object Reference") (OtherActor :type "Actor Object Reference") (OtherComp :type "PrimitiveComponent Object Reference") (OtherBodyIndex :type Integer) (bFromSweep :type Boolean) (SweepResult :type "HitResult Structure (by ref)"))
  (bind _asuovo_bp (cast `/Game/Blueprints/uovoBP` OtherActor))
  (`|SpawnActorFromClass` "/Game/Blueprints/uovoBP.uovoBP_C" (`self.GetTransform` (`|GetArrayItem` (`self.Actor`) (`KismetMathLibrary.RandomIntegerInRange` 0 3))) "Undefined" "OverrideRootScale" null null)
  (`self.K2_DestroyActor` _asuovo_bp))

(fn `UserConstructionScript`)