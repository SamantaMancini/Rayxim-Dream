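; Water slide trigger actor that pushes the Rayxim character along while it overlaps the Box volume.
; On entry it flags Slide, removes ground friction, switches rotation to controller yaw, adds one forward input and sets a fixed velocity along world negative X.
; The push fires only once and ignores the actor's orientation.
; On exit it clears the flag and restores friction and movement-oriented rotation using hard-coded values.
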(event `self.ReceiveTick`
  (params (DeltaSeconds :type "Float (single-precision)")))

(event `self.Box.OnComponentBeginOverlap`
  (params (OverlappedComponent :type "PrimitiveComponent Object Reference") (OtherActor :type "Actor Object Reference") (OtherComp :type "PrimitiveComponent Object Reference") (OtherBodyIndex :type Integer) (bFromSweep :type Boolean) (SweepResult :type "HitResult Structure (by ref)"))
  (bind _asrayxim (cast `/Game/ThirdPersonBP/Rayxim_Animation/Rayxim_2018-12-18-22-44-30` OtherActor))
  (set `/Game/ThirdPersonBP/Rayxim_Animation/Rayxim_2018-12-18-22-44-30.Slide` true _asrayxim)
  (bind _charactermovement (`Character.CharacterMovement` _asrayxim))
  (set `CharacterMovementComponent.bOrientRotationToMovement` false _charactermovement)
  (set `Pawn.bUseControllerRotationYaw` true _asrayxim)
  (set `CharacterMovementComponent.GroundFriction` 0.0 _charactermovement)
  (`Pawn.AddMovementInput` _asrayxim (`self.GetActorForwardVector` _asrayxim) 1.0 false)
  (set `MovementComponent.Velocity` (-1000.0 0.0 0.0) _charactermovement))

(event `self.Box.OnComponentEndOverlap`
  (params (OverlappedComponent :type "PrimitiveComponent Object Reference") (OtherActor :type "Actor Object Reference") (OtherComp :type "PrimitiveComponent Object Reference") (OtherBodyIndex :type Integer))
  (bind _asrayxim (cast `/Game/ThirdPersonBP/Rayxim_Animation/Rayxim_2018-12-18-22-44-30` OtherActor))
  (set `/Game/ThirdPersonBP/Rayxim_Animation/Rayxim_2018-12-18-22-44-30.Slide` false _asrayxim)
  (bind _charactermovement (`Character.CharacterMovement` _asrayxim))
  (set `CharacterMovementComponent.bOrientRotationToMovement` true _charactermovement)
  (set `Pawn.bUseControllerRotationYaw` false _asrayxim)
  (set `CharacterMovementComponent.GroundFriction` 8.0 _charactermovement))

(fn `UserConstructionScript`)