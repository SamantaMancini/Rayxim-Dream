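; Moving platform that slides its mesh along the MovementTrack spline at constant velocity when a Rayxim actor hits it.
; A timeline drives the position along the track, with its play rate set to the inverse of Timemovement.
; CheckHitSide classifies the hit normal by axis and threshold: after a short delay, Up plays the timeline forward and any other detected side reverses it.
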(event `self.ReceiveBeginPlay`
  (`TimelineComponent.SetPlayRate` (`self.Platform`) (/ 1.0 (`self.Timemovement`))))

(event `PlatformMove`
  (bind (_direction _move) (`Timeline|Platform` :!label _label)
    (:`Update`
      (`SceneComponent.K2_SetRelativeLocation` (`self.StaticMesh`) (`SplineComponent.GetLocationAtTime` (`self.MovementTrack`) _move "Local" true) false false))))

(event `Revers`
  (goto _label :!via `Reverse`))

(event `Playrate`
  (`TimelineComponent.SetPlayRate` (`self.Platform`) (/ 1.0 (`self.Timemovement`))))

(event `self.ReceiveHit`
  (params (MyComp :type "PrimitiveComponent Object Reference") (Other :type "Actor Object Reference") (OtherComp :type "PrimitiveComponent Object Reference") (bSelfMoved :type Boolean) (HitLocation :type "Vector Structure") (HitNormal :type "Vector Structure") (NormalImpulse :type "Vector Structure") (Hit :type "HitResult Structure (by ref)"))
  (bind _output_get (set `self.Hit Instigator` Other))
  (cast `/Game/ThirdPersonBP/Rayxim_Animation/Rayxim_2018-12-18-22-44-30` _output_get)
  (`KismetSystemLibrary.Delay` 0.1)
  (switch `/Game/Blueprints/SidePlum` (`self.Check Hit Side` HitNormal 0.1)
    (:`NewEnumerator0`
      (`self.Revers` :!label _label_2)
      (`self.Playrate`))
    (:`NewEnumerator1`
      (goto _label_2))
    (:`NewEnumerator2`
      (goto _label_2))
    (:`NewEnumerator3`
      (goto _label_2))
    (:`NewEnumerator4`
      (`self.PlatformMove`))
    (:`NewEnumerator5`
      (goto _label_2))))

(fn `Check Hit Side`
  (params (Vettore :type "Vector Structure") (CheckOffset :type "Float (double-precision)"))
  (returns (NewParam :type "/Game/Blueprints/SidePlum Enum"))
  (bind _x (.x Vettore))
  (bind _y (.y Vettore))
  (bind _z (.z Vettore))
  (bind _returnvalue (`KismetMathLibrary.FClamp` CheckOffset))
  (bind _returnvalue_2 (* _returnvalue -1.0))
  (if (> _x _returnvalue)
    (return "NewEnumerator0")
    (elif (< _x _returnvalue_2)
      (return "NewEnumerator1")
      (elif (> _y _returnvalue)
        (return "NewEnumerator2")
        (elif (< _y _returnvalue_2)
          (return "NewEnumerator3")
          (elif (> _z _returnvalue)
            (return "NewEnumerator5")
            (elif (< _z _returnvalue_2)
              (return "NewEnumerator4"))))))))

(fn `UserConstructionScript`)