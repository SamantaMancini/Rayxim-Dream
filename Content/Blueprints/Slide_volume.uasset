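; Slide_volume is an overlap volume that puts the Rayxim character into a sliding state while inside it.
; On begin overlap it zeroes ground and braking friction, sets the Slide flag, switches rotation to controller yaw and launches the character additively by its Direction vector.
; On end overlap it clears the flag and restores ground friction and movement-oriented rotation, but leaves braking friction at zero.
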(event `self.ReceiveTick`
  (params (DeltaSeconds :type "Float (single-precision)")))

(event `self.ReceiveActorBeginOverlap`
  (params (OtherActor :type "Actor Object Reference"))
  (bind _asrayxim (cast `/Game/ThirdPersonBP/Rayxim_Animation/Rayxim_2018-12-18-22-44-30` OtherActor))
  (bind _charactermovement (`Character.CharacterMovement` _asrayxim))
  (set `CharacterMovementComponent.GroundFriction` 0.0 _charactermovement)
  (set `CharacterMovementComponent.BrakingFriction` 0.0 _charactermovement)
  (set `/Game/ThirdPersonBP/Rayxim_Animation/Rayxim_2018-12-18-22-44-30.Slide` true _asrayxim)
  (set `CharacterMovementComponent.bOrientRotationToMovement` false _charactermovement)
  (set `Pawn.bUseControllerRotationYaw` true _asrayxim)
  (`Character.LaunchCharacter` _asrayxim (`self.direction`) false false))

(event `CustomEvent`
  (params (DeltaSeconds :type "Float (double-precision)")))

(event `self.ReceiveActorEndOverlap`
  (params (OtherActor :type "Actor Object Reference"))
  (bind _asrayxim (cast `/Game/ThirdPersonBP/Rayxim_Animation/Rayxim_2018-12-18-22-44-30` OtherActor))
  (bind _charactermovement (`Character.CharacterMovement` _asrayxim))
  (set `CharacterMovementComponent.GroundFriction` 8.0 _charactermovement)
  (set `CharacterMovementComponent.BrakingFriction` 0.0 _charactermovement)
  (set `/Game/ThirdPersonBP/Rayxim_Animation/Rayxim_2018-12-18-22-44-30.Slide` false _asrayxim)
  (set `CharacterMovementComponent.bOrientRotationToMovement` true _charactermovement)
  (set `Pawn.bUseControllerRotationYaw` false _asrayxim))

(fn `UserConstructionScript`)