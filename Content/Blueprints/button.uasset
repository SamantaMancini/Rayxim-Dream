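; Pressure-plate button that presses via its "Giù" morph target while something overlaps its box and reacts to actors carrying a configured tag.
; With Conteggio set, it increments or decrements Rayxim_GameMode's counter, updates IsOn through CallOn, and plays Exit when the count reaches four.
; Door plays on press and reverses on release, optionally delayed, whenever Conteggio is off or Porta is also set.
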(event `self.ReceiveBeginPlay`)

(event `self.Box.OnComponentBeginOverlap`
  (params (OverlappedComponent :type "PrimitiveComponent Object Reference") (OtherActor :type "Actor Object Reference") (OtherComp :type "PrimitiveComponent Object Reference") (OtherBodyIndex :type Integer) (bFromSweep :type Boolean) (SweepResult :type "HitResult Structure (by ref)"))
  (`SkeletalMeshComponent.SetMorphTarget` (`self.Button`) "Giù" 1.0 false)
  (if (`self.ActorHasTag` OtherActor (`self.Name`))
    (if (`self.Conteggio?`)
      (`self.Emissivecolor`)
      (if (`self.Porta?`)
        (`MatineeActor.Play` (`self.Door`) :!label _label))
      (else
        (goto _label)))))

(event `self.Box.OnComponentEndOverlap`
  (params (OverlappedComponent :type "PrimitiveComponent Object Reference") (OtherActor :type "Actor Object Reference") (OtherComp :type "PrimitiveComponent Object Reference") (OtherBodyIndex :type Integer))
  (`SkeletalMeshComponent.SetMorphTarget` (`self.Button`) "Giù" 0.0 true)
  (if (`self.ActorHasTag` OtherActor (`self.Name`))
    (if (`self.Conteggio?`)
      (`self.Color`)
      (if (`self.Porta?`)
        (if (`self.Delay?`) :!label _label_2
          (`KismetSystemLibrary.Delay` (`self.Time`)))
        (`MatineeActor.Reverse` (`self.Door`)))
      (else
        (goto _label_2)))))

(event `Color`
  (bind _asrayxim_game_mode (cast `/Game/ThirdPersonBP/Blueprints/Rayxim_Game_mode/Rayxim_GameMode` (`GameplayStatics.GetGameMode`)))
  (`/Game/ThirdPersonBP/Blueprints/Rayxim_Game_mode/Rayxim_GameMode.Decounter` _asrayxim_game_mode)
  (set `self.IsOn` false)
  (`self.On`))

(event `Emissivecolor`
  (bind _asrayxim_game_mode (cast `/Game/ThirdPersonBP/Blueprints/Rayxim_Game_mode/Rayxim_GameMode` (`GameplayStatics.GetGameMode`)))
  (bind _conteggiobutton (`/Game/ThirdPersonBP/Blueprints/Rayxim_Game_mode/Rayxim_GameMode.Counter` _asrayxim_game_mode))
  (set `self.IsOn` true)
  (`self.On`)
  (if (== _conteggiobutton 4)
    (`MatineeActor.Play` (`self.Exit`))))

(fn `UserConstructionScript`)