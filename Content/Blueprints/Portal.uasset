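; Portal actor that sends the Rayxim character to the Heart_of_the_world level.
; On the first overlap by Rayxim, it saves through Rayxim_GameMode, calls Loading on the character, then opens the level after a short delay.
; Separately, any TeensieQueen that begins overlapping the portal's static mesh is destroyed.
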(event `self.ReceiveActorBeginOverlap`
  (params (OtherActor :type "Actor Object Reference"))
  (bind _asrayxim (cast `/Game/ThirdPersonBP/Rayxim_Animation/Rayxim_2018-12-18-22-44-30` OtherActor))
  (`/Engine/EditorBlueprintResources/StandardMacros.DoOnce` false
    (:`Completed`
      (bind _asrayxim_game_mode (cast `/Game/ThirdPersonBP/Blueprints/Rayxim_Game_mode/Rayxim_GameMode` (`GameplayStatics.GetGameMode`)))
      (`/Game/ThirdPersonBP/Blueprints/Rayxim_Game_mode/Rayxim_GameMode.Save` _asrayxim_game_mode)
      (`/Game/ThirdPersonBP/Rayxim_Animation/Rayxim_2018-12-18-22-44-30.Loading` _asrayxim)
      (`KismetSystemLibrary.Delay` 1.5)
      (`GameplayStatics.OpenLevel` "Heart_of_the_world"))))

(event `self.StaticMesh.OnComponentBeginOverlap`
  (params (OverlappedComponent :type "PrimitiveComponent Object Reference") (OtherActor :type "Actor Object Reference") (OtherComp :type "PrimitiveComponent Object Reference") (OtherBodyIndex :type Integer) (bFromSweep :type Boolean) (SweepResult :type "HitResult Structure (by ref)"))
  (bind _asteensie_queen (cast `/Game/personaggi/Teensie/Queen_teensie/TeensieQueen` OtherActor))
  (`self.K2_DestroyActor` _asteensie_queen))

(fn `UserConstructionScript`)