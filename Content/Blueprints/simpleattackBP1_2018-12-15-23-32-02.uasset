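; Projectile actor for a simple attack that deals damage and explodes on contact.
; Both a hit and an overlap on its Sphere apply the projectile damage to the other actor, then spawn an explosion effect and sound.
; Each impact briefly pulses a RadialForce before destroying the actor.
; Without contact, it destroys itself after a fixed lifetime started at BeginPlay.
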(event `self.ReceiveBeginPlay`
  (`KismetSystemLibrary.Delay` 6.0)
  (`self.K2_DestroyActor`))

(event `self.Sphere.OnComponentHit`
  (params (HitComponent :type "PrimitiveComponent Object Reference") (OtherActor :type "Actor Object Reference") (OtherComp :type "PrimitiveComponent Object Reference") (NormalImpulse :type "Vector Structure") (Hit :type "HitResult Structure (by ref)"))
  (`GameplayStatics.ApplyDamage` OtherActor (`self.Dannoproiettile`) null self)
  (`GameplayStatics.SpawnEmitterAtLocation` "/Game/StarterContent/Particles/P_Explosion.P_Explosion" (`SceneComponent.K2_GetComponentLocation` (`self.Sphere`)))
  (`GameplayStatics.PlaySoundAtLocation` "/Game/Enemies/Nymplix/terrexpl_Cue.terrexpl_Cue" (`.Location` (`GameplayStatics.BreakHitResult` Hit)) (struct) 1.0 1.0 0.0 null null null)
  (`ActorComponent.Activate` (`self.RadialForce`) false)
  (`KismetSystemLibrary.Delay` 0.2)
  (`ActorComponent.Deactivate` (`self.RadialForce`))
  (`self.K2_DestroyActor`))

(event `self.Sphere.OnComponentBeginOverlap`
  (params (OverlappedComponent :type "PrimitiveComponent Object Reference") (OtherActor :type "Actor Object Reference") (OtherComp :type "PrimitiveComponent Object Reference") (OtherBodyIndex :type Integer) (bFromSweep :type Boolean) (SweepResult :type "HitResult Structure (by ref)"))
  (`GameplayStatics.ApplyDamage` OtherActor (`self.Dannoproiettile`) null self)
  (`GameplayStatics.SpawnEmitterAtLocation` "/Game/StarterContent/Particles/P_Explosion.P_Explosion" (`SceneComponent.K2_GetComponentLocation` (`self.Sphere`)))
  (`GameplayStatics.PlaySoundAtLocation` "/Game/Enemies/Nymplix/terrexpl_Cue.terrexpl_Cue" (`self.K2_GetActorLocation`) (struct) 1.0 1.0 0.0 null null null)
  (`ActorComponent.Activate` (`self.RadialForce`) false)
  (`KismetSystemLibrary.Delay` 0.2)
  (`ActorComponent.Deactivate` (`self.RadialForce`))
  (`self.K2_DestroyActor`))

(fn `UserConstructionScript`)