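; Zombie chicken enemy character that plays a rise montage, starts its Behavior Tree through ZombieChickenController, then sets itself a short lifespan.
; It faces a LookAtTarget on Tick, set by either a Path event or a Chase function that also moves it toward the player.
; Overlapping Rayxim damages them, and either that or a simpleattackBP1 hit stops its AI, ragdolls it and resets the despawn timer.
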(event `self.ReceiveBeginPlay`
  (bind _returnvalue (`self.PlayAnimMontage` "/Game/Enemies/ZombieChickens/Show_zombie_Montage.Show_zombie_Montage"))
  (`KismetSystemLibrary.Delay` _returnvalue)
  (bind _aszombie_chicken_controller (cast `/Game/Enemies/ZombieChickens/ZombieChickenController` (`self.GetController`)))
  (`/Game/Enemies/ZombieChickens/ZombieChickenController.Initialize` _aszombie_chicken_controller self (`self.BehaviorTree`) (`self.Blackboard`))
  (`self.SetLifeSpan` 2.0))

(event `self.ReceiveTick`
  (params (DeltaSeconds :type "Float (single-precision)"))
  (bind _lookattarget (`self.LookAtTarget`))
  (bind (_returnvalue_roll _returnvalue_pitch _returnvalue_yaw) (`KismetMathLibrary.BreakRotator` (`KismetMathLibrary.FindLookAtRotation` (`self.K2_GetActorLocation`) (`self.K2_GetActorLocation` _lookattarget))))
  (`/Engine/EditorBlueprintResources/StandardMacros.IsValid` _lookattarget
    (:`Is Valid`
      (`self.K2_SetActorRotation` (`KismetMathLibrary.MakeRotator` _returnvalue_roll 0.0 _returnvalue_yaw)))))

(event `/Game/Enemies/EnemyUtilities.Path`
  (params (PathTrack :type "Actor Object Reference"))
  (set `self.LookAtTarget` PathTrack))

(event `self.CapsuleComponent.OnComponentBeginOverlap`
  (params (OverlappedComponent :type "PrimitiveComponent Object Reference") (OtherActor :type "Actor Object Reference") (OtherComp :type "PrimitiveComponent Object Reference") (OtherBodyIndex :type Integer) (bFromSweep :type Boolean) (SweepResult :type "HitResult Structure (by ref)"))
  (bind _mesh (`self.Mesh`))
  (cast `/Game/Blueprints/simpleattackBP1_2018-12-15-23-32-02` OtherActor)
  (bind _aszombie_chicken_controller (cast `/Game/Enemies/ZombieChickens/ZombieChickenController` (`self.GetController`)))
  (`/Game/Enemies/ZombieChickens/ZombieChickenController.StopLogic` _aszombie_chicken_controller)
  (`SkeletalMeshComponent.SetAllBodiesSimulatePhysics` _mesh true)
  (`MovementComponent.StopMovementImmediately` (`self.CharacterMovement`))
  (`self.SetLifeSpan` 1.5)
  (`PrimitiveComponent.SetCollisionProfileName` _mesh "Ragdoll"))

(event `self.ReceiveActorBeginOverlap`
  (params (OtherActor :type "Actor Object Reference"))
  (bind _mesh (`self.Mesh`))
  (bind _asrayxim (cast `/Game/ThirdPersonBP/Rayxim_Animation/Rayxim_2018-12-18-22-44-30` OtherActor))
  (bind _aszombie_chicken_controller (cast `/Game/Enemies/ZombieChickens/ZombieChickenController` (`self.GetController`)))
  (`/Game/Enemies/ZombieChickens/ZombieChickenController.StopLogic` _aszombie_chicken_controller)
  (`GameplayStatics.ApplyDamage` _asrayxim 10.0 null self)
  (`self.SetLifeSpan` 1.5)
  (`SkeletalMeshComponent.SetAllBodiesSimulatePhysics` _mesh true)
  (`MovementComponent.StopMovementImmediately` (`self.CharacterMovement`))
  (`PrimitiveComponent.SetCollisionProfileName` _mesh "Ragdoll"))

(event `Player`
  (`|AIMoveTo` self (0.0 0.0 0.0) (`GameplayStatics.GetPlayerCharacter` 0) 500.0))

(fn `Chase`
  (returns (Output_Get :type "Actor Object Reference"))
  (`self.Player`)
  (bind _output_get (set `self.LookAtTarget` (`GameplayStatics.GetPlayerCharacter` 0)))
  (return _output_get))

(fn `UserConstructionScript`)